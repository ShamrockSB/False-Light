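; BP_Energy is a Blueprint that holds an energy pool, starting empty with a maximum set in the construction script.
; AddEnergy raises the current value, clamped between zero and the maximum, and fires OnEnergyChanged.
; UseEnergy succeeds only when the amount is at least the current energy, then stores amount minus current and fires the same event.
; That comparison and subtraction appear reversed for a spend operation.
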(event `self.ReceiveBeginPlay`)

(fn `AddEnergy`
  (params (Amount :type Integer))
  ;[0 0.1354 0.15 0.5] Add energy logic
  (set `self.CurrentEnergy` (`KismetMathLibrary.Clamp` (+ Amount (`self.CurrentEnergy`)) 0 (`self.MaxEnergy`)))
  (`self.OnEnergyChanged` (`self.MaxEnergy`) (`self.CurrentEnergy`)))

(fn `UseEnergy`
  (params (Amount :type Integer))
  (returns (Success :type Boolean))
  ;[0.04886 0.02746 0.15 0.5] UseEnergy
  (if (>= Amount (`self.CurrentEnergy`))
    (set `self.CurrentEnergy` (- Amount (`self.CurrentEnergy`)))
    (`self.OnEnergyChanged` (`self.MaxEnergy`) (`self.CurrentEnergy`))
    (return true)
    (else
      (return false))))

(fn `UserConstructionScript`
  (set `self.MaxEnergy` 3)
  (set `self.CurrentEnergy` 0))