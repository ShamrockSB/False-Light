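; BP_PowerSwitch is an interactable switch that the side-scrolling character powers on by spending a full energy bar.
; A trigger overlap enables player input and marks the player as nearby, and leaving it disables input again.
; Pressing E while nearby checks that Energy equals MaxEnergy, then zeroes it, sets HasPower and toggles three Niagara effects.
; HasPower makes activation one-time, with later presses only printing a message.
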(event `self.ReceiveBeginPlay`)

(event `Key|E`
  (params (Key :type "Key Structure"))
  (:`Pressed`
    (if (`self.hasPower`)
      (`KismetSystemLibrary.PrintString` "Already turned on")
      (elif (`self.bIsPlayerNearby`)
        (`KismetSystemLibrary.PrintString` "E Pressed")
        (bind _asbp_side_scrolling_character (cast `/Game/_SB/Blueprints/BP_SideScrollingCharacter` (`GameplayStatics.GetPlayerCharacter` 0)))
        (if (== (`/Game/_SB/Blueprints/BP_SideScrollingCharacter.Energy` _asbp_side_scrolling_character) (`/Game/_SB/Blueprints/BP_SideScrollingCharacter.MaxEnergy` _asbp_side_scrolling_character))
          (set `/Game/_SB/Blueprints/BP_SideScrollingCharacter.Energy` 0 _asbp_side_scrolling_character)
          (set `self.hasPower` true)
          (`ActorComponent.ToggleActive` (`self.Niagara1`))
          (`ActorComponent.ToggleActive` (`self.Niagara`))
          (`ActorComponent.ToggleActive` (`self.Niagara2`)))))))

(event `self.Trigger.OnComponentBeginOverlap`
  (params (OverlappedComponent :type "PrimitiveComponent Object Reference") (OtherActor :type "Actor Object Reference") (OtherComp :type "PrimitiveComponent Object Reference") (OtherBodyIndex :type Integer) (bFromSweep :type Boolean) (SweepResult :type "HitResult Structure (by ref)"))
  (cast `/Game/_SB/Blueprints/BP_SideScrollingCharacter` OtherActor)
  (`self.EnableInput` (`GameplayStatics.GetPlayerController` 0))
  (set `self.bIsPlayerNearby` true))

(event `self.Trigger.OnComponentEndOverlap`
  (params (OverlappedComponent :type "PrimitiveComponent Object Reference") (OtherActor :type "Actor Object Reference") (OtherComp :type "PrimitiveComponent Object Reference") (OtherBodyIndex :type Integer))
  (cast `/Game/_SB/Blueprints/BP_SideScrollingCharacter` OtherActor)
  (`self.DisableInput` (`GameplayStatics.GetPlayerController` 0))
  (set `self.bIsPlayerNearby` false))

(fn `UserConstructionScript`)