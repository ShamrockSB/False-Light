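; Beacon door actor that sends the side-scrolling player to Lvl_Main once their energy is full.
; A box overlap with the player character enables the actor's input and flags the player as nearby, and leaving it reverses both.
; Pressing E while nearby checks that Energy equals MaxEnergy, then clears IsNight on the BP_LevelOrder game instance before opening the level.
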(event `Key|E`
  (params (Key :type "Key Structure"))
  (:`Pressed`
    (if (`self.bPlayerNearby`)
      (`KismetSystemLibrary.PrintString` "E Pressed")
      (bind _asbp_side_scrolling_character (cast `/Game/_SB/Blueprints/BP_SideScrollingCharacter` (`GameplayStatics.GetPlayerCharacter` 0)))
      (if (== (`/Game/_SB/Blueprints/BP_SideScrollingCharacter.Energy` _asbp_side_scrolling_character) (`/Game/_SB/Blueprints/BP_SideScrollingCharacter.MaxEnergy` _asbp_side_scrolling_character))
        (bind _asbp_level_order (cast `/Game/_SB/Blueprints/BP_LevelOrder` (`GameplayStatics.GetGameInstance`)))
        (set `/Game/_SB/Blueprints/BP_LevelOrder.bIsNight` false _asbp_level_order)
        (`GameplayStatics.OpenLevel` "Lvl_Main")))))

(event `self.Box.OnComponentBeginOverlap`
  (params (OverlappedComponent :type "PrimitiveComponent Object Reference") (OtherActor :type "Actor Object Reference") (OtherComp :type "PrimitiveComponent Object Reference") (OtherBodyIndex :type Integer) (bFromSweep :type Boolean) (SweepResult :type "HitResult Structure (by ref)"))
  (cast `/Game/_SB/Blueprints/BP_SideScrollingCharacter` OtherActor)
  (`self.EnableInput` (`GameplayStatics.GetPlayerController` 0))
  (set `self.bPlayerNearby` true))

(event `self.Box.OnComponentEndOverlap`
  (params (OverlappedComponent :type "PrimitiveComponent Object Reference") (OtherActor :type "Actor Object Reference") (OtherComp :type "PrimitiveComponent Object Reference") (OtherBodyIndex :type Integer))
  (cast `/Game/_SB/Blueprints/BP_SideScrollingCharacter` OtherActor)
  (`self.DisableInput` (`GameplayStatics.GetPlayerController` 0))
  (set `self.bPlayerNearby` false))

(fn `UserConstructionScript`)