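; Enemy AI pawn for a side-scrolling game that is drawn to lit light zones and restarts the level when it touches the player.
; Each tick it finds the nearest BP_LightZone and, only if that zone's light is on, stores it as the current target and issues an AI move toward it.
; Its Box overlap with BP_SideScrollingCharacter reopens the current level.
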(event `self.ReceiveTick`
  (params (DeltaSeconds :type "Float (single-precision)"))
  (bind _outactors (`GameplayStatics.GetAllActorsOfClass` "/Game/_SB/Blueprints/Lights/BP_LightZone.BP_LightZone_C"))
  (bind _asbp_light_zone (cast `/Game/_SB/Blueprints/Lights/BP_LightZone` (`.ReturnValue` (`GameplayStatics.FindNearestActor` (`self.K2_GetActorLocation`) _outactors))))
  (if (`/Game/_SB/Blueprints/Lights/BP_LightZone.bIsLightOn` _asbp_light_zone)
    (bind _output_get (set `self.currentTargetLight` _asbp_light_zone))
    (`|AIMoveTo` self (`self.K2_GetActorLocation` _asbp_light_zone) _output_get)))

(event `self.ReceiveBeginPlay`)

(event `self.Box.OnComponentBeginOverlap`
  (params (OverlappedComponent :type "PrimitiveComponent Object Reference") (OtherActor :type "Actor Object Reference") (OtherComp :type "PrimitiveComponent Object Reference") (OtherBodyIndex :type Integer) (bFromSweep :type Boolean) (SweepResult :type "HitResult Structure (by ref)"))
  (cast `/Game/_SB/Blueprints/BP_SideScrollingCharacter` OtherActor)
  (bind _returnvalue (`GameplayStatics.GetCurrentLevelName` true))
  (`GameplayStatics.OpenLevel` (`KismetStringLibrary.Conv_StringToName` _returnvalue)))

(fn `UserConstructionScript`)