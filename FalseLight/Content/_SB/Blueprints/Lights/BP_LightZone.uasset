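; BP_LightZone is a clickable light that the player switches on and off by spending and reclaiming character energy.
; Clicking the Cube toggles IsLightOn: switching on requires and takes one Energy from the BP_SideScrollingCharacter, and switching off returns it.
; Tick polls that flag every frame and sets the SpotLight intensity to either lit or dark.
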(event `self.ReceiveTick`
  (params (DeltaSeconds :type "Float (single-precision)"))
  ; Comment
  (if (`self.bIsLightOn`)
    (`LightComponent.SetIntensity` (`self.SpotLight`) 450.0)
    (else
      (`LightComponent.SetIntensity` (`self.SpotLight`) 0.0))))

(event `self.Cube.OnClicked`
  (params (TouchedComponent :type "PrimitiveComponent Object Reference") (ButtonPressed :type "Key Structure"))
  (bind _asbp_side_scrolling_character (cast `/Game/_SB/Blueprints/BP_SideScrollingCharacter` (`GameplayStatics.GetPlayerCharacter` 0)))
  (if (`self.bIsLightOn`)
    (set `self.bIsLightOn` (not (`self.bIsLightOn`)))
    (bind _energy (`/Game/_SB/Blueprints/BP_SideScrollingCharacter.Energy` _asbp_side_scrolling_character))
    (`/Engine/EditorBlueprintResources/StandardMacros.IncrementInt` _energy)
    (elif (> _energy 0)
      (set `self.bIsLightOn` (not (`self.bIsLightOn`)))
      (`/Engine/EditorBlueprintResources/StandardMacros.DecrementInt` _energy))))

(fn `UserConstructionScript`)